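; BP_MovePoint1 is a clickable lane-switch marker for BP_RunCharacter, moving the character sideways to a fixed Y position.
; Each Tick it stays a fixed X distance ahead of the player on that lane, hiding once the character's Y is nonzero.
; Releasing a click on its mesh plays a timeline that lerps the character onto the lane, keeping its current X.
; The logic to show it again is unconnected.
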(event OnReleased(StaticMesh)
  (params (TouchedComponent :type Primitive%20Component%20Object%20Reference) (ButtonReleased :type Key%20Structure :default "None"))
  (bind _character (Variables|Default|GetCharacter))
  (bind _alpha (Timeline|타임라인_0 PlayFromStart)
    (:Update
      (Transformation|SetActorLocation _character (Math|Vector|Lerp(Vector) (Transformation|GetActorLocation _character) (Math|Vector|MakeVector (.x (Transformation|GetActorLocation (Game|GetPlayerCharacter 0))) 325.0 90.08931) _alpha) false false))))

(event EventBeginPlay
  (bind _asbp_run_character (Utilities|Casting|CastToBP_RunCharacter (Game|GetPlayerCharacter 0)))
  (Variables|Default|SetCharacter _asbp_run_character))

(event Collision|EventActorBeginOverlap
  (params (OtherActor :type Actor%20Object%20Reference)))

(event EventTick
  (params (DeltaSeconds :type Float%20%28single-precision%29))
  (Transformation|SetActorLocation (Math|Vector|MakeVector (+ (.x (Transformation|GetActorLocation (Game|GetPlayerCharacter 0))) 3e+02) 325.0 2e+01) false false)
  (if (!= (.y (Transformation|GetActorLocation (Variables|Default|GetCharacter))) 0.0)
    (Rendering|SetActorHiddenInGame true)))

(fn ConstructionScript)